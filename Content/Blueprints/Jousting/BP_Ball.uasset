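; BP_Ball is a physics ball actor in the Jousting content that resets to its starting transform after the player character hits it.
; It saves its transform on BeginPlay, and when a BP_FirstPersonCharacter hits its mesh it plays an impact sound and waits ten seconds.
; It then teleports back and briefly toggles physics simulation off and on, which restarts it at the start position.
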(event OnComponentHit(StaticMeshComponent)
  (params (HitComponent :type Primitive%20Component%20Object%20Reference) (OtherActor :type Actor%20Object%20Reference) (OtherComp :type Primitive%20Component%20Object%20Reference) (NormalImpulse :type Vector :default "0, 0, 0") (Hit :type Hit%20Result%20Structure%20%28by%20ref%29))
  (Utilities|Casting|CastToBP_FirstPersonCharacter OtherActor)
  (Audio|PlaySoundatLocation "/Game/UI/impact_1.impact_1" (Transformation|GetActorLocation) "0, 0, 0" 1.0 1.0 0.0 0 0 0 0)
  (Utilities|FlowControl|Delay 1e+01)
  (Transformation|SetActorTransform (Variables|Default|Getstartpos) false true)
  (Physics|SetSimulatePhysics (Variables|Debug|GetStaticMeshComponent) false)
  (Utilities|FlowControl|Delay 0.2)
  (Physics|SetSimulatePhysics (Variables|Debug|GetStaticMeshComponent) true))

(event EventBeginPlay
  (Variables|Default|Setstartpos (Transformation|GetActorTransform)))

(event Collision|EventActorBeginOverlap
  (params (OtherActor :type Actor%20Object%20Reference)))

(event EventTick
  (params (DeltaSeconds :type Float%20%28single-precision%29)))

(fn ConstructionScript)