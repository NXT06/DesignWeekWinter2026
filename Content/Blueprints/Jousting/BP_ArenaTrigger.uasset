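; Arena trigger that starts and ends a two-player jousting match.
; Box overlaps track which player controllers and characters are inside, firing Stop, Waiting or Start dispatchers as the count changes.
; With two players, after a short delay it sets GameOn and teleports them to spawn offsets with opposite yaw.
; Tick polls BP_Splitscreen for an unhorsed player, then fires GameOver and reloads Lvl_Playground after a delay.
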(event OnComponentBeginOverlap(Box)
  (params (OverlappedComponent :type Primitive%20Component%20Object%20Reference) (OtherActor :type Actor%20Object%20Reference) (OtherComp :type Primitive%20Component%20Object%20Reference) (OtherBodyIndex :type Integer) (bFromSweep :type Boolean) (SweepResult :type Hit%20Result%20Structure%20%28by%20ref%29))
  (bind _players (Variables|Default|GetPlayers))
  (bind _returnvalue (Utilities|Array|Length _players))
  (if (not (Variables|Default|GetGameOn))
    (bind _asbp_first_person_character (Utilities|Casting|CastToBP_FirstPersonCharacter OtherActor))
    (if (not (Utilities|Array|ContainsItem _players (Game|GetInstigatorController _asbp_first_person_character)))
      (Utilities|Array|Add (Variables|Default|GetPlayerCharacters) _asbp_first_person_character)
      (Utilities|Array|AddUnique _players (Game|GetInstigatorController _asbp_first_person_character))
      (Development|PrintString (Utilities|String|ToString(Integer) _returnvalue))
      (switch int _returnvalue
        (:0
          (Default|CallEDStop))
        (:1
          (Default|CallEDWaiting))
        (:2
          (Default|CallEDStart)
          (Utilities|FlowControl|Delay 3.2)
          (CallFunction|CEJoust))))))

(event OnComponentEndOverlap(Box)
  (params (OverlappedComponent :type Primitive%20Component%20Object%20Reference) (OtherActor :type Actor%20Object%20Reference) (OtherComp :type Primitive%20Component%20Object%20Reference) (OtherBodyIndex :type Integer))
  (bind _players (Variables|Default|GetPlayers))
  (if (not (Variables|Default|GetGameOn))
    (bind _asbp_first_person_character (Utilities|Casting|CastToBP_FirstPersonCharacter OtherActor))
    (Utilities|Array|RemoveItem _players (Game|GetInstigatorController _asbp_first_person_character))
    (Utilities|Array|RemoveItem (Variables|Default|GetPlayerCharacters) _asbp_first_person_character)
    (Development|PrintString (Utilities|String|ToString(Integer) (Utilities|Array|Length _players)))
    (switch int (Utilities|Array|Length (Variables|Default|GetPlayers))
      (:0
        (Default|CallEDStop))
      (:1
        (Default|CallEDWaiting))
      (:2
        (Default|CallEDStart)
        (Utilities|FlowControl|Delay 3.2)
        (CallFunction|CEJoust)))))

(event Custom|CE_Joust
  (Variables|Default|SetGameOn true)
  (for (_array_element _array_index) (Variables|Default|GetPlayerCharacters)
    (if (> _array_index 0)
      (Transformation|SetActorLocationAndRotation _array_element (+ (Transformation|GetActorLocation) (Utilities|Array|Get(acopy) (Variables|Default|GetSpawns) _array_index)) "0.000000,90.000000,0.000000" false true)
      (else
        (Transformation|SetActorLocationAndRotation _array_element (+ (Transformation|GetActorLocation) (Utilities|Array|Get(acopy) (Variables|Default|GetSpawns) _array_index)) "0.000000,-90.000000,0.000000" false true)))))

(event Custom|CE_Reset
  (Actor|GetAllActorsOfClass "/Script/Engine.PlayerStart"))

(event EventBeginPlay)

(event Collision|EventActorBeginOverlap
  (params (OtherActor :type Actor%20Object%20Reference)))

(event EventTick
  (params (DeltaSeconds :type Float%20%28single-precision%29))
  (if (Variables|Default|GetGameOn)
    (bind _asbp_splitscreen (Utilities|Casting|CastToBP_Splitscreen (Game|GetGameMode)))
    (if (!= (Variables|/Game/FirstPerson/Blueprints/BP_Splitscreen.BP_Splitscreen_C|GetUnhorsedPlayer _asbp_splitscreen) -5)
      (Variables|Default|SetGameOn false)
      (Default|CallEDGameOver)
      (Utilities|FlowControl|Delay 3.0)
      (Game|OpenLevel(byObjectReference) "/Game/FirstPerson/Lvl_Playground.Lvl_Playground"))))

(fn ConstructionScript)