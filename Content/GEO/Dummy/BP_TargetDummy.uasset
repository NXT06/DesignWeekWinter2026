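; BP_TargetDummy is a target dummy that gets knocked over when BP_FirstPersonCharacter hits it, then respawns.
; It stores its starting transform on BeginPlay.
; A character hit on its component clears the constraint mode, enables gravity and applies a radial impulse at the impact point.
; After a short delay it spawns a fresh dummy at the stored transform and destroys itself, printing debug text along the way.
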(event OnComponentHit(1)
  (params (HitComponent :type Primitive%20Component%20Object%20Reference) (OtherActor :type Actor%20Object%20Reference) (OtherComp :type Primitive%20Component%20Object%20Reference) (NormalImpulse :type Vector :default "0, 0, 0") (Hit :type Hit%20Result%20Structure%20%28by%20ref%29))
  (bind _1 (Variables|Default|Get1))
  (Utilities|Casting|CastToBP_FirstPersonCharacter OtherActor)
  (Development|PrintText "Hello")
  (Class|PrimitiveComponent|SetConstraintMode _1 "None")
  (Physics|SetEnableGravity _1 true)
  (Physics|AddRadialImpulse _1 (.ImpactPoint (Collision|BreakHitResult Hit)) 1e+02 7e+02 "RIF_Constant" false)
  (Utilities|FlowControl|Delay 5.0)
  (Development|PrintText "Hello")
  (Transformation|SetActorTransform (Variables|Default|Getstartpos) false true)
  (Game|SpawnActorfromClass "BP_TargetDummy_C" (Variables|Default|Getstartpos) "Undefined" "MultiplyWithRoot" 0 0)
  (Actor|DestroyActor))

(event EventBeginPlay
  (Variables|Default|Setstartpos (Transformation|GetActorTransform)))

(event Collision|EventActorBeginOverlap
  (params (OtherActor :type Actor%20Object%20Reference)))

(event EventTick
  (params (DeltaSeconds :type Float%20%28single-precision%29)))

(fn ConstructionScript)